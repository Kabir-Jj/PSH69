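; BP_Foonga is an enemy character that moves back and forth along its right vector, turning around at obstacles.
; Each tick it applies movement input in TraceDirection, then line-traces the Visibility channel TraceDistance ahead along that same axis.
; A blocking hit drives a FlipFlop that sets TraceDirection alternately to -1 and 1, reversing both movement and trace.
; The trace has debug drawing left on.
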(event EventTick
  (params (DeltaSeconds :type Float%20%28single-precision%29))
  (bind _returnvalue (Transformation|GetActorLocation))
  (Utilities|FlowControl|Sequence
    (:then_0
      (Pawn|Input|AddMovementInput (* (Transformation|GetActorRightVector) (Variables|Default|GetTraceDirection)) 1.0 false))
    (:then_1
      (bind _outhit (Collision|LineTraceByChannel _returnvalue (+ _returnvalue (* (* (Transformation|GetActorRightVector) (Variables|Default|GetTraceDirection)) (Variables|Default|GetTraceDistance))) "TraceTypeQuery1" false 0 "ForDuration"))
      (if (.bBlockingHit (Collision|BreakHitResult _outhit))
        (Utilities|FlowControl|FlipFlop
          (:A
            (Variables|Default|SetTraceDirection -1.0))
          (:B
            (Variables|Default|SetTraceDirection 1.0)))))))

(fn ConstructionScript
  (|CallParentFunction))