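; BP_Door is an interactable door that opens only for a player carrying a key, by removing itself from the world.
; Its Interact event casts the interacting actor to BP_PlayerCharacter, checks HasKey, and destroys the door actor when true.
; The key is only checked, not consumed, and nothing happens for other actors or players without a key.
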(event EventBeginPlay
  (|CallParentFunction) ; This node is disabled and will not be called.\nDrag off pins to build functionality.
)

(event Collision|EventActorBeginOverlap
  (params (OtherActor :type Actor%20Object%20Reference))
  (|CallParentFunction OtherActor) ; This node is disabled and will not be called.\nDrag off pins to build functionality.
)

(event EventTick
  (params (DeltaSeconds :type Float%20%28single-precision%29))
  (|CallParentFunction DeltaSeconds) ; This node is disabled and will not be called.\nDrag off pins to build functionality.
)

(event EventInteract
  (params (InteractingActor :type Actor%20Object%20Reference))
  (bind _asbp_player_character (Utilities|Casting|CastToBP_PlayerCharacter InteractingActor))
  (if (Variables|/Game/_Game/Blueprints/Characters/PlayerCharacter/BP_PlayerCharacter.BP_PlayerCharacter_C|GetHasKey _asbp_player_character)
    (Actor|DestroyActor)))

(fn ConstructionScript
  (|CallParentFunction))