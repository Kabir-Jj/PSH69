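; BP_MeshPopulator is a construction-script actor that lines a spline with copies of a chosen mesh, filed with the castle wall Blueprints.
; Spacing comes from the mesh's bounding-box X size plus an Offset, and the spline length divided by it sets the instance count.
; Each copy is added to an InstancedStaticMesh at unit scale, rotated to face the next sample point along the spline.
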(event EventBeginPlay)

(event Collision|EventActorBeginOverlap
  (params (OtherActor :type Actor%20Object%20Reference)))

(event EventTick
  (params (DeltaSeconds :type Float%20%28single-precision%29)))

(fn ConstructionScript
  (Components|StaticMesh|SetStaticMesh (Variables|Default|GetInstancedStaticMesh) (Variables|Default|GetPlacedMesh))
  (bind _spacing (Utilities|CalculateSpacing))
  (bind _output_get (Variables|Default|SetNoOfInstances (Math|Float|Floor (/ (Spline|GetSplineLength (Variables|Default|GetSpline)) _spacing))))
  (for _index (range 0 _output_get)
    (Components|InstancedStaticMesh|AddInstance (Variables|Default|GetInstancedStaticMesh) (Math|Transform|MakeTransform (CallFunction|GetLocationatIndex _index) (Math|Rotator|MakeRotfromX (- (CallFunction|GetLocationatIndex (+ _index 1)) (CallFunction|GetLocationatIndex _index)))))))

(fn GetLocationatIndex
  (params (Index :type Integer))
  (return (Spline|GetLocationatDistanceAlongSpline (Variables|Default|GetSpline) (* Index (Variables|Default|GetSpacing)) "Local")))